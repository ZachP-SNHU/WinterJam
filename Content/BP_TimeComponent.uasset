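; Actor component that records its owner's recent motion so the actor can be rewound or frozen in time.
; A looping timer, configured from the BP_TimeWarp game mode, either records, rewinds or holds the owner according to its state flags.
; Recording keeps a capped rolling buffer of transform and root physics velocities.
; Rewind interpolates backwards through these snapshots, consuming them, while freeze disables physics simulation and reapplies the latest one.
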(event `self.ReceiveBeginPlay`
  (`self.Setup` (`GameplayStatics.GetGameMode`))
  (`self.Start TimeTracker`)
  (`KismetSystemLibrary.K2_SetTimerDelegate` (delegate `TimeCollection`) (`self.TrackFrequency`) true))

(event `TimeCollection`
  (if (`self.bIsRewinding`)
    (`self.Reverse Time`)
    (elif (`self.bIsFrozen`)
      (`self.PauseTime`)
      (else
        (`self.RecordTime`)))))

(fn `ApplyTime`
  (params (TimeApplied :type "/Game/TimeWarp/Data/Struct_TimeSnap Structure"))
  (bind _ownerroot (`self.OwnerRoot`))
  (`Actor.K2_SetActorTransform` (`self.GetOwner`) TimeApplied_Transform_2_1CAF5C3A457F618690237C91A8A17027 false false)
  (`PrimitiveComponent.SetPhysicsLinearVelocity` _ownerroot TimeApplied_LinearVelocity_6_C3991EB0495D5249D24BFDB6205CE7A0 false "None")
  (`PrimitiveComponent.SetPhysicsAngularVelocityInRadians` _ownerroot TimeApplied_AngularVelocity_8_C52DF2B64F185235AB2B4C90F5EBB487 false "None"))

(fn `ApplyTimeInterpolated`
  (params (TimeSnapEnd :type "/Game/TimeWarp/Data/Struct_TimeSnap Structure") (TimeSnapBegin :type "/Game/TimeWarp/Data/Struct_TimeSnap Structure"))
  (bind _ownerroot (`self.OwnerRoot`))
  (bind _progress (`self.Progress`))
  (`Actor.K2_SetActorTransform` (`self.GetOwner`) (`KismetMathLibrary.TLerp` TimeSnapBegin_Transform_2_1CAF5C3A457F618690237C91A8A17027 TimeSnapEnd_Transform_2_1CAF5C3A457F618690237C91A8A17027 _progress) false false)
  (`PrimitiveComponent.SetPhysicsLinearVelocity` _ownerroot (`KismetMathLibrary.VLerp` TimeSnapBegin_LinearVelocity_6_C3991EB0495D5249D24BFDB6205CE7A0 TimeSnapEnd_LinearVelocity_6_C3991EB0495D5249D24BFDB6205CE7A0 _progress) false "None")
  (`PrimitiveComponent.SetPhysicsAngularVelocityInRadians` _ownerroot (`KismetMathLibrary.VLerp` TimeSnapBegin_AngularVelocity_8_C52DF2B64F185235AB2B4C90F5EBB487 TimeSnapEnd_AngularVelocity_8_C52DF2B64F185235AB2B4C90F5EBB487 _progress) false "None"))

(fn `Pause Physics`
  (params (ShouldPause :type Boolean) (PhysicsObject :type Boolean))
  (bind _ownerroot (`self.OwnerRoot`))
  (if PhysicsObject
    (if ShouldPause
      (`PrimitiveComponent.SetSimulatePhysics` _ownerroot false :!label _label)
      (else
        (`PrimitiveComponent.SetSimulatePhysics` _ownerroot true)))
    (else
      (goto _label))))

(fn `PauseTime`
  (bind _timesnaps (`self.timeSnaps`))
  (`self.Pause Physics` true (`self.Physics Object`))
  (`self.ApplyTime` (`|GetArrayItem` _timesnaps (`KismetArrayLibrary.Array_LastIndex` _timesnaps))))

(fn `RecordTime`
  (bind _ownerroot (`self.OwnerRoot`))
  (if (>= (`KismetArrayLibrary.Array_Length` (`self.timeSnaps`)) (`self.MaxSnaps`))
    (`KismetArrayLibrary.Array_Remove` (`self.timeSnaps`)))
  (bind _returnvalue (`PrimitiveComponent.GetPhysicsLinearVelocity` _ownerroot "None"))
  (`KismetArrayLibrary.Array_Add` (`self.timeSnaps`) (make `/Game/TimeWarp/Data/Struct_TimeSnap` (`Actor.GetTransform` (`self.GetOwner`)) _returnvalue (`PrimitiveComponent.GetPhysicsAngularVelocityInRadians` _ownerroot "None"))))

(fn `Reverse Time`
  (bind _timesnaps (`self.timeSnaps`))
  (bind _timesnaps_2 (`self.timeSnaps`))
  (bind _timesnaps_3 (`self.timeSnaps`))
  (bind _timesnaps_4 (`self.timeSnaps`))
  (bind _returnvalue (`KismetArrayLibrary.Array_LastIndex` _timesnaps_2))
  (bind _returnvalue_2 (- _returnvalue 1))
  (if (`KismetArrayLibrary.Array_IsValidIndex` _timesnaps_2 _returnvalue_2)
    (set `self.Progress` (`KismetMathLibrary.FClamp` (+ (`self.Progress`) (`self.RewindSpeed`))))
    (`self.ApplyTimeInterpolated` (`|GetArrayItem` _timesnaps _returnvalue_2) (`|GetArrayItem` _timesnaps _returnvalue))
    (if (>= (`self.Progress`) 1.0)
      (set `self.Progress` 0.0)
      (`KismetArrayLibrary.Array_Remove` _timesnaps_3 (`KismetArrayLibrary.Array_LastIndex` _timesnaps_3)))
    (else
      (`self.ApplyTime` (`|GetArrayItem` _timesnaps_4 (`KismetArrayLibrary.Array_LastIndex` _timesnaps_4)))
      (set `self.bIsRewinding` false))))

(fn `Setup`
  (params (GameMode :type "GameModeBase Object Reference"))
  (bind _asbp_time_warp (cast `/Game/Blueprint/BP_TimeWarp` GameMode))
  (set `self.MaxTimeTracked` (`/Game/Blueprint/BP_TimeWarp.MaxTimeTracked` _asbp_time_warp))
  (set `self.TrackFrequency` (`/Game/Blueprint/BP_TimeWarp.TrackFrequency` _asbp_time_warp))
  (bind _asprimitive_component (cast `PrimitiveComponent` (`Actor.RootComponent` (`self.GetOwner`))))
  (set `self.OwnerRoot` _asprimitive_component))

(fn `Start TimeTracker`
  (set `self.MaxSnaps` (/ (`self.MaxTimeTracked`) (`self.TrackFrequency`))))

(fn `Stop Manipulation`
  (bind _timesnaps (`self.timeSnaps`))
  (set `self.bIsRewinding` false)
  (set `self.bIsFrozen` false)
  (`self.Pause Physics` false)
  (`self.ApplyTime` (`|GetArrayItem` _timesnaps (`KismetArrayLibrary.Array_LastIndex` _timesnaps))))