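; BP_Door is a two-panel sliding door that opens for NPC-tagged actors and responds to time manipulation.
; Collision overlaps play or reverse the OpenDoor timeline, which slides the upper and lower panels apart vertically, unless BPTimeComponent is frozen.
; TimePause stops the timeline and applies a time-controlled material, while TimeReverse toggles rewinding or freezing.
; TimeEnd restores the saved materials and resumes opening or closing based on IsOpening.
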(event `self.Collision.OnComponentBeginOverlap`
  (params (OverlappedComponent :type "PrimitiveComponent Object Reference") (OtherActor :type "Actor Object Reference") (OtherComp :type "PrimitiveComponent Object Reference") (OtherBodyIndex :type Integer) (bFromSweep :type Boolean) (SweepResult :type "HitResult Structure (by ref)"))
  (if (`self.ActorHasTag` OtherActor "NPC")
    (`self.DoorOpen`)))

(event `self.Collision.OnComponentEndOverlap`
  (params (OverlappedComponent :type "PrimitiveComponent Object Reference") (OtherActor :type "Actor Object Reference") (OtherComp :type "PrimitiveComponent Object Reference") (OtherBodyIndex :type Integer))
  (`self.DoorClose`))

(event `DoorOpen`
  (set `self.Is Opening` true)
  (if (not (`/Game/Blueprint/BP_TimeComponent.bIsFrozen` (`self.BP_TimeComponent`)))
    (bind (_direction _open_close) (`Timeline|Open Door` :`NewTime` (stale `/Game/Blueprint/BPI_TimeWarp.TimeReverse` ReverseSpeed) :!label _label)
      (:`Update`
        (bind _returnvalue (`KismetMathLibrary.Lerp` 0.0 93.0 _open_close))
        (`SceneComponent.K2_SetRelativeLocation` (`self.DoorUpper`) (`KismetMathLibrary.MakeVector` 0.0 0.0 _returnvalue) false false)
        (`SceneComponent.K2_SetRelativeLocation` (`self.DoorLower`) (`KismetMathLibrary.MakeVector` 0.0 0.0 (* _returnvalue -1.0)) false false))
      (:`Finished`
        (set `self.Is Opening` false)))))

(event `DoorClose`
  (if (not (`/Game/Blueprint/BP_TimeComponent.bIsFrozen` (`self.BP_TimeComponent`)))
    (goto _label :!via `Reverse`)))

(event `/Game/Blueprint/BPI_TimeWarp.TimePause`
  (bind _bp_timecomponent (`self.BP_TimeComponent`))
  (if (not (`/Game/Blueprint/BP_TimeComponent.bIsFrozen` _bp_timecomponent))
    (set `/Game/Blueprint/BP_TimeComponent.bIsFrozen` true _bp_timecomponent)
    (bind _output_get (set `self.Original Materials` (`MeshComponent.GetMaterials` (`self.DoorUpper`))))
    (for (_ _array_index) _output_get
      (`PrimitiveComponent.SetMaterial` (`self.DoorUpper`) _array_index "/Game/Materials/M_TimeControlled.M_TimeControlled")
      (`PrimitiveComponent.SetMaterial` (`self.DoorLower`) _array_index "/Game/Materials/M_TimeControlled.M_TimeControlled")
      (goto _label :!via `Stop`))))

(event `/Game/Blueprint/BPI_TimeWarp.TimeReverse`
  (params (ReverseSpeed :type "Float (double-precision)"))
  (bind _bp_timecomponent (`self.BP_TimeComponent`))
  (if (> ReverseSpeed 0.0)
    (set `/Game/Blueprint/BP_TimeComponent.bIsRewinding` true _bp_timecomponent)
    (if (`self.Is Opening`)
      (goto _label :!via `SetNewTime`)
      (else
        (goto _label :!via `SetNewTime`)))
    (else
      (set `/Game/Blueprint/BP_TimeComponent.bIsFrozen` true _bp_timecomponent)
      (set `/Game/Blueprint/BP_TimeComponent.bIsRewinding` false _bp_timecomponent))))

(event `/Game/Blueprint/BPI_TimeWarp.TimeEnd`
  (`/Game/Blueprint/BP_TimeComponent.Stop Manipulation` (`self.BP_TimeComponent`))
  (for (_array_element _array_index) (`self.Original Materials`)
    (`PrimitiveComponent.SetMaterial` (`self.DoorUpper`) _array_index _array_element)
    (`PrimitiveComponent.SetMaterial` (`self.DoorLower`) _array_index _array_element)
    (if (`self.Is Opening`)
      (`self.DoorOpen`)
      (else
        (`self.DoorClose`)))))

(fn `UserConstructionScript`)