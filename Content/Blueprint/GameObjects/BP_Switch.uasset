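; BP_Switch is a lever switch that BP_TimeWarpCharacter can flip while inside its overlap sphere, which also shows an interact widget.
; Interact, or Reset without the range check, alternately plays and reverses a timeline that rotates the lever.
; Each finish alternates the On state, light material and sound, calling Toggle only when switching off.
; Toggle passes actors tagged by Targets to Activate or Deactivate, both empty events here.
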(event `/Game/Blueprint/BPI_Interact.Interact`
  (bind _returnvalue (`self.K2_GetActorLocation`))
  (bind _sphere (`self.Sphere`))
  (if (`self.CanInteract`)
    (`/Engine/EditorBlueprintResources/StandardMacros.FlipFlop` :!label _label
      (:`A`
        (bind (_direction _switch) (`Timeline|Flip Switch` :!label _label_2)
          (:`Update`
            (`SceneComponent.K2_SetRelativeRotation` (`self.Lever`) (`KismetMathLibrary.MakeRotator` 0.0 (`KismetMathLibrary.Lerp` -50.0 -120.0 _switch)) false false))
          (:`Finished`
            (`/Engine/EditorBlueprintResources/StandardMacros.FlipFlop`
              (:`A`
                (set `self.On` false)
                (`PrimitiveComponent.SetMaterial` _sphere 0 "/Game/Materials/M_CameraLens.M_CameraLens")
                (`GameplayStatics.PlaySoundAtLocation` "/Engine/VREditor/Sounds/UI/Dockable_Window_Close.Dockable_Window_Close" _returnvalue (struct) 1.0 1.0 0.0 null null null null)
                (`self.Toggle`))
              (:`B`
                (set `self.On` true)
                (`GameplayStatics.PlaySoundAtLocation` "/Engine/VREditor/Sounds/UI/Dockable_Window_Open.Dockable_Window_Open" _returnvalue (struct) 1.0 1.0 0.0 null null null null)
                (`PrimitiveComponent.SetMaterial` _sphere 0 "/Game/Materials/M_RedLight.M_RedLight"))))))
      (:`B`
        (goto _label_2 :!via `Reverse`)))))

(event `Reset`
  (goto _label))

(event `self.ReceiveBeginPlay`
  (bind _returnvalue (`|CreateWidget` "/Game/UI/P_Interact.P_Interact_C"))
  (set `self.Interact Widget` _returnvalue)
  (`GameplayStatics.PrimeSound` "/Engine/VREditor/Sounds/UI/Dockable_Window_Close.Dockable_Window_Close")
  (`GameplayStatics.PrimeSound` "/Engine/VREditor/Sounds/UI/Dockable_Window_Open.Dockable_Window_Open"))

(event `Toggle`
  (if (`self.On`)
    (bind _outactors (`GameplayStatics.GetAllActorsWithTag` (`self.Targets`)))
    (for _array_element _outactors
      (`self.Deactivate` _array_element))
    (else
      (bind _outactors_2 (`GameplayStatics.GetAllActorsWithTag` (`self.Targets`)))
      (for _array_element_2 _outactors_2
        (`self.Activate` _array_element_2)))))

(event `self.Sphere1.OnComponentBeginOverlap`
  (params (OverlappedComponent :type "PrimitiveComponent Object Reference") (OtherActor :type "Actor Object Reference") (OtherComp :type "PrimitiveComponent Object Reference") (OtherBodyIndex :type Integer) (bFromSweep :type Boolean) (SweepResult :type "HitResult Structure (by ref)"))
  (cast `/Game/PlayerCharacter/BP_TimeWarpCharacter` OtherActor)
  (`UserWidget.AddToViewport` (`self.Interact Widget`) 0)
  (set `self.CanInteract` true))

(event `Deactivate`
  (params (Actor :type "Actor Object Reference")))

(event `self.Sphere1.OnComponentEndOverlap`
  (params (OverlappedComponent :type "PrimitiveComponent Object Reference") (OtherActor :type "Actor Object Reference") (OtherComp :type "PrimitiveComponent Object Reference") (OtherBodyIndex :type Integer))
  (cast `/Game/PlayerCharacter/BP_TimeWarpCharacter` OtherActor)
  (`Widget.RemoveFromParent` (`self.Interact Widget`))
  (set `self.CanInteract` false))

(event `Activate`
  (params (Actor :type "Actor Object Reference")))

(fn `UserConstructionScript`)