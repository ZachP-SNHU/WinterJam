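; BP_Sensor is a detection sensor that raises the alarm and alerts nearby NPC drones when it detects the player.
; Detection plays a point-light flash timeline with sound: a single flash for lasers, otherwise a triple flash that can be cancelled if the player leaves.
; When the flash finishes, it starts BP_Alarm actors, re-arms, and writes alarm state and its location to the blackboards of BP_NPC pawns found by sphere overlap.
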(event `Detect Player`
  (params (Player :type "Actor Object Reference"))
  (if (and (`self.ActorHasTag` Player "Player") (not (`self.hasDetected`)))
    (set `self.hasDetected` true)
    (`self.Flash` false)))

(event `TriggerDrones`
  (`self.GetLocalDrones`)
  (for _array_element (stale `GetLocalDrones` _output_get)
    (bind _asnpc_aic (cast `/Game/AI/NPC_AIC` (`AIBlueprintHelperLibrary.GetAIController` _array_element)))
    (`/Game/AI/NPC_AIC.SetBlackBoardValues` _asnpc_aic true (`self.SensorLocation`))))

(event `GetLocalDrones`
  (bind _outactors (`KismetSystemLibrary.SphereOverlapActors` (`self.SensorLocation`) 2000.0 (`|MakeArray` "ObjectTypeQuery3" :!type "EObjectTypeQuery Enum") "/Game/AI/BP_NPC.BP_NPC_C"))
  (bind _output_get (set `self.TriggeredDrones` _outactors)))

(event `Flash`
  (params (PlayerLeft :type Boolean))
  (if (`self.isLaser`)
    (bind (_direction _intensity) (`Timeline|Flash Once` :!via `PlayFromStart`)
      (:`Update`
        (`LightComponent.SetIntensity` (`self.PointLight`) (`KismetMathLibrary.Lerp` 0.0 300000.0 _intensity)))
      (:`Finished`
        (bind _outactors (`GameplayStatics.GetAllActorsOfClass` "/Game/Blueprint/GameObjects/Traps/BP_Alarm.BP_Alarm_C" :!label _label))
        (`/Game/Blueprint/GameObjects/Traps/BP_Alarm.Start Alarm` _outactors)
        (set `self.hasDetected` false)
        (`self.TriggerDrones`))
      (:`Sound`
        (`GameplayStatics.PlaySoundAtLocation` (`self.DetectionSound`) (`self.K2_GetActorLocation`) (struct) 1.0 1.0 0.0 "/Game/Audio/SFX/SA_Sensor.SA_Sensor" null null null :!label _label_2)))
    (elif PlayerLeft
      (`self.Cancel`)
      (bind (_direction_2 _intensity_2) (`Timeline|Triple Flash` :!via `SetNewTime` :!label _label_3)
        (:`Update`
          (`LightComponent.SetIntensity` (`self.PointLight`) (`KismetMathLibrary.Lerp` 0.0 300000.0 _intensity_2)))
        (:`Finished`
          (goto _label))
        (:`Sound`
          (goto _label_2)))
      (else
        (goto _label_3 :!via `PlayFromStart`)))))

(event `Cancel`
  (`LightComponent.SetIntensity` (`self.PointLight`) 0.0)
  (goto _label_3 :!via `Stop`))

(fn `UserConstructionScript`
  (set `self.SensorLocation` (`self.K2_GetActorLocation`)))