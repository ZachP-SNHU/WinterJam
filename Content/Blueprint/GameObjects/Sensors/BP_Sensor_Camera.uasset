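; A security camera sensor that sweeps left and right and detects the time-warp player character entering its detection zone.
; A timeline yaws the pivot at a fixed down angle, with a FlipFlop reversing each pass.
; Unless frozen, overlap triggers flash and detection logic.
; Time events, tracked through BPTimeComponent, pause the sweep with a material swap, restore and resume it, or rewind it by lerping timeline position.
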(event `self.ReceiveBeginPlay`
  ;[1 1 1] Camera Swivel
  (`KismetSystemLibrary.Delay` (`self.StartDelay`))
  (bind (_direction _rotatemovement) (`Timeline|Rotate` :`NewTime` (`self.CurrentTimelineTime`) :!label _label)
    (:`Update`
      (`SceneComponent.K2_SetRelativeRotation` (`self.Pivot`) (`KismetMathLibrary.MakeRotator` 0.0 (`self.Down Angle`) (`KismetMathLibrary.Lerp` 120.0 60.0 _rotatemovement)) false false))
    (:`Finished`
      (bind _isa (`/Engine/EditorBlueprintResources/StandardMacros.FlipFlop`) ; A is left to right
        (:`A`
          (goto _label))
        (:`B`
          (goto _label :!via `Reverse`))))))

(event `/Game/Blueprint/BPI_TimeWarp.TimePause`
  (bind _bp_timecomponent (`self.BP_TimeComponent`))
  ;[1 1 1] Time Pause
  (set `self.CurrentTimelineTime` (`TimelineComponent.GetPlaybackPosition` (`self.Rotate`)))
  (if (not (`/Game/Blueprint/BP_TimeComponent.bIsFrozen` _bp_timecomponent))
    (set `/Game/Blueprint/BP_TimeComponent.bIsFrozen` true _bp_timecomponent)
    (bind _output_get (set `self.Original Materials` (`MeshComponent.GetMaterials` (`self.CameraHousing`))))
    (for (_ _array_index) _output_get
      (`PrimitiveComponent.SetMaterial` (`self.CameraHousing`) _array_index "/Game/Materials/M_TimeControlled.M_TimeControlled")
      (goto _label :!via `Stop`))))

(event `RestartCamera`
  ;[1 1 1] Camera Swivel
  (if (stale `self.ReceiveBeginPlay` _isa)
    (goto _label)
    (else
      (goto _label :!via `Reverse`))))

(event `/Game/Blueprint/BPI_TimeWarp.TimeEnd`
  ;[1 1 1] Time Resume
  (`/Game/Blueprint/BP_TimeComponent.Stop Manipulation` (`self.BP_TimeComponent`))
  (for (_array_element _array_index) (`self.Original Materials`)
    (`PrimitiveComponent.SetMaterial` (`self.CameraHousing`) _array_index _array_element)
    (`self.RestartCamera`)))

(event `self.DetectionZone.OnComponentBeginOverlap`
  (params (OverlappedComponent :type "PrimitiveComponent Object Reference") (OtherActor :type "Actor Object Reference") (OtherComp :type "PrimitiveComponent Object Reference") (OtherBodyIndex :type Integer) (bFromSweep :type Boolean) (SweepResult :type "HitResult Structure (by ref)"))
  ;[1 1 1] Player Detection
  (bind _asbp_time_warp_character (cast `/Game/PlayerCharacter/BP_TimeWarpCharacter` OtherActor))
  (bind _output_get (set `self.PlayerInZone` true))
  (if (not (`/Game/Blueprint/BP_TimeComponent.bIsFrozen` (`self.BP_TimeComponent`)))
    (`self.Flash` (not _output_get))
    (if (`self.PlayerInZone`)
      (`self.Detect Player` _asbp_time_warp_character))))

(event `/Game/Blueprint/BPI_TimeWarp.TimeReverse`
  (params (ReverseSpeed :type "Float (double-precision)"))
  (bind _bp_timecomponent (`self.BP_TimeComponent`))
  (if (> ReverseSpeed 0.0)
    (set `/Game/Blueprint/BP_TimeComponent.bIsRewinding` true _bp_timecomponent)
    (bind _output_get (set `/Game/Blueprint/BP_TimeComponent.RewindSpeed` ReverseSpeed _bp_timecomponent))
    (if (stale `self.ReceiveBeginPlay` _isa)
      (set `self.CurrentTimelineTime` (`KismetMathLibrary.Lerp` (`self.CurrentTimelineTime`) 0.0 _output_get))
      (goto _label :!via `SetNewTime`)
      (else
        (set `self.CurrentTimelineTime` (`KismetMathLibrary.Lerp` (`self.CurrentTimelineTime`) 5.0 _output_get))
        (goto _label :!via `SetNewTime`)))
    (else
      (set `/Game/Blueprint/BP_TimeComponent.bIsFrozen` true _bp_timecomponent)
      (set `/Game/Blueprint/BP_TimeComponent.bIsRewinding` false _bp_timecomponent))))

(event `self.DetectionZone.OnComponentEndOverlap`
  (params (OverlappedComponent :type "PrimitiveComponent Object Reference") (OtherActor :type "Actor Object Reference") (OtherComp :type "PrimitiveComponent Object Reference") (OtherBodyIndex :type Integer))
  ;[1 1 1] Player Detection
  (cast `/Game/PlayerCharacter/BP_TimeWarpCharacter` OtherActor)
  (set `self.PlayerInZone` false)
  (`self.Cancel`))

(fn `UserConstructionScript`
  (`parent.UserConstructionScript`))