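; A sliding door that opens automatically when the player's time-warp character enters its collision volume and closes when it leaves.
; Overlap events cast to BP_TimeWarpCharacter, then call the DoorOpen or DoorClose events.
; A single OpenDoor timeline plays forward or in reverse, lerping the relative Z of upper and lower panels so they split vertically apart.
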(event `self.Collision.OnComponentBeginOverlap`
  (params (OverlappedComponent :type "PrimitiveComponent Object Reference") (OtherActor :type "Actor Object Reference") (OtherComp :type "PrimitiveComponent Object Reference") (OtherBodyIndex :type Integer) (bFromSweep :type Boolean) (SweepResult :type "HitResult Structure (by ref)"))
  (cast `/Game/PlayerCharacter/BP_TimeWarpCharacter` OtherActor)
  (`self.DoorOpen`))

(event `self.Collision.OnComponentEndOverlap`
  (params (OverlappedComponent :type "PrimitiveComponent Object Reference") (OtherActor :type "Actor Object Reference") (OtherComp :type "PrimitiveComponent Object Reference") (OtherBodyIndex :type Integer))
  (cast `/Game/PlayerCharacter/BP_TimeWarpCharacter` OtherActor)
  (`self.DoorClose`))

(event `DoorOpen`
  (bind (_direction _open_close) (`Timeline|Open Door` :!label _label)
    (:`Update`
      (`SceneComponent.K2_SetRelativeLocation` (`self.DoorUpper`) (`KismetMathLibrary.MakeVector` 0.0 0.0 (`KismetMathLibrary.Lerp` 0.0 135.0 _open_close)) false false)
      (`SceneComponent.K2_SetRelativeLocation` (`self.DoorLower`) (`KismetMathLibrary.MakeVector` 0.0 0.0 (`KismetMathLibrary.Lerp` 0.0 -90.0 _open_close)) false false))))

(event `DoorClose`
  (goto _label :!via `Reverse`))

(fn `UserConstructionScript`)