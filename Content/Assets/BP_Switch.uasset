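; BP_Switch is an interactable lever switch that shows or hides all actors tagged with its GroupNumber, toggling their collision too.
; Overlap by BP_TimeWarpCharacter on Sphere1 displays the interact widget and enables Interact.
; Interact alternately plays and reverses a timeline that pitches the lever.
; When the timeline finishes, a second FlipFlop swaps the indicator sphere's material and On state, then Deactivate applies that state to the group.
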(event `/Game/BPI_Interact.Interact`
  (bind _sphere (`self.Sphere`))
  (if (`self.CanInteract`)
    (`/Engine/EditorBlueprintResources/StandardMacros.FlipFlop`
      (:`A`
        (bind (_direction _switch) (`Timeline|Flip Switch` :!label _label)
          (:`Update`
            (`SceneComponent.K2_SetRelativeRotation` (`self.Lever`) (`KismetMathLibrary.MakeRotator` 0.0 (`KismetMathLibrary.Lerp` -50.0 -120.0 _switch)) false false))
          (:`Finished`
            (`/Engine/EditorBlueprintResources/StandardMacros.FlipFlop`
              (:`A`
                (`PrimitiveComponent.SetMaterial` _sphere 0 "/Game/Materials/M_CameraLens.M_CameraLens")
                (set `self.On` false))
              (:`B`
                (`PrimitiveComponent.SetMaterial` _sphere 0 "/Game/Materials/M_RedLight.M_RedLight")
                (set `self.On` true)))
            (`self.Deactivate`))))
      (:`B`
        (goto _label :!via `Reverse`)))))

(event `self.ReceiveBeginPlay`
  (bind _returnvalue (`|CreateWidget` "/Game/UI/P_Interact.P_Interact_C"))
  (set `self.Interact Widget` _returnvalue))

(event `Deactivate`
  (if (`self.On`)
    (bind _outactors (`GameplayStatics.GetAllActorsWithTag` (`self.Group Number`)))
    (for _array_element _outactors
      (`self.SetActorHiddenInGame` _array_element false)
      (`self.SetActorEnableCollision` _array_element true))
    (else
      (bind _outactors_2 (`GameplayStatics.GetAllActorsWithTag` (`self.Group Number`)))
      (for _array_element_2 _outactors_2
        (`self.SetActorHiddenInGame` _array_element_2 true)
        (`self.SetActorEnableCollision` _array_element_2 false)))))

(event `self.Sphere1.OnComponentBeginOverlap`
  (params (OverlappedComponent :type "PrimitiveComponent Object Reference") (OtherActor :type "Actor Object Reference") (OtherComp :type "PrimitiveComponent Object Reference") (OtherBodyIndex :type Integer) (bFromSweep :type Boolean) (SweepResult :type "HitResult Structure (by ref)"))
  (cast `/Game/PlayerCharacter/BP_TimeWarpCharacter` OtherActor)
  (`UserWidget.AddToViewport` (`self.Interact Widget`) 0)
  (set `self.CanInteract` true))

(event `self.Sphere1.OnComponentEndOverlap`
  (params (OverlappedComponent :type "PrimitiveComponent Object Reference") (OtherActor :type "Actor Object Reference") (OtherComp :type "PrimitiveComponent Object Reference") (OtherBodyIndex :type Integer))
  (cast `/Game/PlayerCharacter/BP_TimeWarpCharacter` OtherActor)
  (`Widget.RemoveFromParent` (`self.Interact Widget`))
  (set `self.CanInteract` false))

(fn `UserConstructionScript`)