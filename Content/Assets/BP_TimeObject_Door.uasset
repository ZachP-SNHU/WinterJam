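; Sliding door time object that opens when a BP_TimeWarpCharacter enters its DetectEntity volume and closes when it leaves.
; A single DoorOpen timeline moves the upper and lower halves apart vertically in opposite directions.
; TimePause stops that timeline and TimeReverse plays it backwards, so time manipulation affects the door's motion, with closing also reusing the reversed timeline.
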(event `DoorOpen`
  (bind (_direction _open_close) (`Timeline|Door Open` :!label _label)
    (:`Update`
      (bind _returnvalue (`KismetMathLibrary.Lerp` 0.0 90.0 _open_close))
      (`SceneComponent.K2_SetRelativeLocation` (`self.DoorLower`) (`KismetMathLibrary.MakeVector` 0.0 0.0 (* _returnvalue -1.0)) false false)
      (`SceneComponent.K2_SetRelativeLocation` (`self.DoorUpper`) (`KismetMathLibrary.MakeVector` 0.0 0.0 _returnvalue) false false))))

(event `/Game/Blueprint/BPI_TimeWarp.TimePause`
  (goto _label :!via `Stop`))

(event `/Game/Blueprint/BPI_TimeWarp.TimeReverse`
  (params (ReverseSpeed :type "Float (double-precision)"))
  (goto _label :!via `Reverse`))

(event `DoorClose`
  (goto _label :!via `Reverse`))

(event `self.DetectEntity.OnComponentEndOverlap`
  (params (OverlappedComponent :type "PrimitiveComponent Object Reference") (OtherActor :type "Actor Object Reference") (OtherComp :type "PrimitiveComponent Object Reference") (OtherBodyIndex :type Integer))
  (cast `/Game/Blueprint/BP_TimeWarpCharacter` OtherActor)
  (`self.DoorClose`))

(event `self.DetectEntity.OnComponentBeginOverlap`
  (params (OverlappedComponent :type "PrimitiveComponent Object Reference") (OtherActor :type "Actor Object Reference") (OtherComp :type "PrimitiveComponent Object Reference") (OtherBodyIndex :type Integer) (bFromSweep :type Boolean) (SweepResult :type "HitResult Structure (by ref)"))
  (cast `/Game/Blueprint/BP_TimeWarpCharacter` OtherActor)
  (`self.DoorOpen`))

(fn `UserConstructionScript`
  (`parent.UserConstructionScript`))