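; BP_Sensor_Camera is a security camera sensor that sweeps back and forth and detects the player.
; After a start delay, the Rotate timeline swings the Pivot's yaw across a fixed arc at the DownAngle pitch.
; A FlipFlop on the timeline's finish alternates Play and Reverse to keep the sweep going.
; When a BP_TimeWarpCharacter begins overlapping DetectionZone, it is passed to DetectPlayer.
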(event `self.ReceiveBeginPlay`
  (bind _down_angle (`self.Down Angle`))
  (`KismetSystemLibrary.Delay` (`self.Duration`))
  (bind (_direction _rotatemovement) (`Timeline|Rotate` :!label _label)
    (:`Update`
      (`SceneComponent.K2_SetRelativeRotation` (`self.Pivot`) (`KismetMathLibrary.RLerp` (`KismetMathLibrary.MakeRotator` 0.0 _down_angle 110.0) (`KismetMathLibrary.MakeRotator` 0.0 _down_angle 70.0) _rotatemovement) false false))
    (:`Finished`
      (`/Engine/EditorBlueprintResources/StandardMacros.FlipFlop`
        (:`A`
          (goto _label))
        (:`B`
          (goto _label :!via `Reverse`))))))

(event `self.DetectionZone.OnComponentBeginOverlap`
  (params (OverlappedComponent :type "PrimitiveComponent Object Reference") (OtherActor :type "Actor Object Reference") (OtherComp :type "PrimitiveComponent Object Reference") (OtherBodyIndex :type Integer) (bFromSweep :type Boolean) (SweepResult :type "HitResult Structure (by ref)"))
  (bind _asbp_time_warp_character (cast `/Game/Blueprint/BP_TimeWarpCharacter` OtherActor))
  (`self.Detect Player` _asbp_time_warp_character))

(fn `UserConstructionScript`
  (`parent.UserConstructionScript`))