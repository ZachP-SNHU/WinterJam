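; BP_Sensor is a sensor actor that raises the alarm when it detects the player.
; Its DetectPlayer event checks for the Player tag and latches HasDetected, so it responds only once.
; Detection plays an attenuated sound at the sensor, calls StartAlarm on every BP_Alarm in the level, and runs a timeline that drives the point light's intensity.
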(event `Detect Player`
  (params (Player :type "Actor Object Reference"))
  (if (and (`self.ActorHasTag` Player "Player") (not (`self.hasDetected`)))
    (set `self.hasDetected` true)
    (`GameplayStatics.PlaySoundAtLocation` (`self.DetectionSound`) (`self.K2_GetActorLocation`) (struct) 1.0 1.0 0.0 "/Game/Audio/SFX/SA_Sensor.SA_Sensor" null null null)
    (bind _outactors (`GameplayStatics.GetAllActorsOfClass` "/Game/Assets/BP_Alarm.BP_Alarm_C"))
    (`/Game/Assets/BP_Alarm.Start Alarm` _outactors)
    (bind (_direction _intensity) (`Timeline|Timeline`)
      (:`Update`
        (`LightComponent.SetIntensity` (`self.PointLight`) (`KismetMathLibrary.Lerp` 0.0 300000.0 _intensity))))))

(fn `UserConstructionScript`)