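; BP_TimeObject_SensorBase is a sensor base Blueprint that raises the alarm when it detects a player.
; DetectPlayer latches on the first player passing an actor tag check, plays a detection sound at the sensor and calls StartAlarm on the BP_Alarm actors in the level.
; It then calls Flash, where a timeline drives the point light's intensity.
; Nothing in this graph calls DetectPlayer or resets the detection flag.
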(event `Detect Player`
  (params (Player :type "/Game/PlayerCharacter/BP_TimeWarpCharacter Object Reference"))
  (if (and (`self.ActorHasTag` Player "None") (not (`self.hasDetected`)))
    (set `self.hasDetected` true)
    (`GameplayStatics.PlaySoundAtLocation` (`self.DetectionSound`) (`self.K2_GetActorLocation`) (struct) 1.0 1.0 0.0 null null null null)
    (bind _outactors (`GameplayStatics.GetAllActorsOfClass` "/Game/Assets/Traps/BP_Alarm.BP_Alarm_C"))
    (`/Game/Assets/Traps/BP_Alarm.Start Alarm` _outactors)
    (`self.Flash`)))

(event `Flash`
  (bind (_direction _intensity) (`Timeline|Flash PointLight`)
    (:`Update`
      (`LightComponent.SetIntensity` (`self.PointLight`) (`KismetMathLibrary.Lerp` 0.0 300000.0 _intensity)))))

(fn `UserConstructionScript`
  (`parent.UserConstructionScript`))