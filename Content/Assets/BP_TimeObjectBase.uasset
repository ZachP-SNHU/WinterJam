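; Base Blueprint for objects that can be paused or rewound by time manipulation.
; TimePause, TimeReverse and TimeEnd events drive a BPTimeComponent's frozen, rewinding and speed state, with TimeEnd stopping the manipulation.
; Pausing caches the static mesh's materials and swaps every slot to M_TimeControlled, and TimeEnd restores the cached set.
; TimeReverse treats a non-positive speed as a freeze and leaves materials untouched.
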(event `self.ReceiveBeginPlay`)

(event `/Game/BPI_TimeWarp.TimePause`
  (bind _bp_timecomponent (`self.BP_TimeComponent`))
  (if (not (`/Game/BP_TimeComponent.bIsFrozen` _bp_timecomponent))
    (set `/Game/BP_TimeComponent.bIsFrozen` true _bp_timecomponent)
    (bind _output_get (set `self.Original Materials` (`MeshComponent.GetMaterials` (`self.StaticMesh`))))
    (for (_ _array_index) _output_get
      (`PrimitiveComponent.SetMaterial` (`self.StaticMesh`) _array_index "/Game/Materials/M_TimeControlled.M_TimeControlled"))))

(event `/Game/BPI_TimeWarp.TimeReverse`
  (params (ReverseSpeed :type "Float (double-precision)"))
  (bind _bp_timecomponent (`self.BP_TimeComponent`))
  (if (> ReverseSpeed 0.0)
    (set `/Game/BP_TimeComponent.bIsRewinding` true _bp_timecomponent)
    (set `/Game/BP_TimeComponent.RewindSpeed` ReverseSpeed _bp_timecomponent)
    (else
      (set `/Game/BP_TimeComponent.bIsFrozen` true _bp_timecomponent)
      (set `/Game/BP_TimeComponent.bIsRewinding` false _bp_timecomponent))))

(event `/Game/BPI_TimeWarp.TimeEnd`
  (`/Game/BP_TimeComponent.Stop Manipulation` (`self.BP_TimeComponent`))
  (for (_array_element _array_index) (`self.Original Materials`)
    (`PrimitiveComponent.SetMaterial` (`self.StaticMesh`) _array_index _array_element)))

(fn `UserConstructionScript`)