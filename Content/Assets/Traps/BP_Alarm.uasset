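; BP_Alarm is an alarm actor that plays a siren sound and rotating spotlights when triggered.
; StartAlarm spawns MS_Alarm at the actor's location and activates RotatingMovement, while StopAlarm fades the sound out and deactivates it, both guarded by AlarmActive.
; RotatingMovement's activation events drive both spotlights' visibility, with the Reset flag serving as the visible state on activation.
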(event `Start Alarm`
  (if (not (`self.AlarmActive`))
    (bind _returnvalue (`GameplayStatics.SpawnSoundAtLocation` "/Game/Audio/SFX/MS_Alarm.MS_Alarm" (`self.K2_GetActorLocation`) (struct) 1.0 1.0 0.0 null null))
    (set `self.AlarmSound` _returnvalue)
    (set `self.AlarmActive` true)
    (`ActorComponent.Activate` (`self.RotatingMovement`) true)))

(event `Stop Alarm`
  (if (`self.AlarmActive`)
    (`AudioComponent.FadeOut` (`self.AlarmSound`) 1.0 0.0 "Linear")
    (set `self.AlarmActive` false)
    (`ActorComponent.Deactivate` (`self.RotatingMovement`))))

(event `self.RotatingMovement.OnComponentActivated`
  (params (Component :type "ActorComponent Object Reference") (bReset :type Boolean))
  (`SceneComponent.SetVisibility` (`self.SpotLight`) bReset false)
  (`SceneComponent.SetVisibility` (`self.SpotLight1`) bReset false))

(event `self.RotatingMovement.OnComponentDeactivated`
  (params (Component :type "ActorComponent Object Reference"))
  (`SceneComponent.SetVisibility` (`self.SpotLight`) false false)
  (`SceneComponent.SetVisibility` (`self.SpotLight1`) false false))

(fn `UserConstructionScript`)