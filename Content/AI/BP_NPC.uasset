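; BP_NPC is an NPC that ends the game when the player's BP_TimeWarpCharacter touches its Hitbox, by calling GameOver on that character.
; The construction script caches the sensor point light's color as the default.
; ChangeLightColor and ResetLight switch both sensor lights (spot and point) between the player-detected color and that default, with no callers in this Blueprint.
; NpcPath is an empty function here, and Tick is unused.
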(event `self.ReceiveBeginPlay`)

(event `self.hitbox.OnComponentBeginOverlap`
  (params (OverlappedComponent :type "PrimitiveComponent Object Reference") (OtherActor :type "Actor Object Reference") (OtherComp :type "PrimitiveComponent Object Reference") (OtherBodyIndex :type Integer) (bFromSweep :type Boolean) (SweepResult :type "HitResult Structure (by ref)"))
  (bind _asbp_time_warp_character (cast `/Game/PlayerCharacter/BP_TimeWarpCharacter` OtherActor))
  (`/Game/PlayerCharacter/BP_TimeWarpCharacter.GameOver` _asbp_time_warp_character))

(fn `ChangeLightColor`
  (bind _player_detected_color (`self.player detected color`))
  (`LightComponent.SetLightColor` (`self.SensorSpotLight`) _player_detected_color true)
  (`LightComponent.SetLightColor` (`self.SensorPointLight`) _player_detected_color true))

(fn `NpcPath`
  (returns (Path :type "/Game/AI/BP_SplinePath Object Reference"))
  (return null))

(fn `ResetLight`
  (bind _defaultcolor (`self.DefaultColor`))
  (`LightComponent.SetLightColor` (`self.SensorSpotLight`) _defaultcolor true)
  (`LightComponent.SetLightColor` (`self.SensorPointLight`) _defaultcolor true))

(fn `UserConstructionScript`
  (set `self.DefaultColor` (`LightComponentBase.GetLightColor` (`self.SensorPointLight`))))